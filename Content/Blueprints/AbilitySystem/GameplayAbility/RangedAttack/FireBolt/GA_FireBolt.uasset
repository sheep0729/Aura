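; GA_FireBolt is a ranged fire bolt gameplay ability that casts a projectile toward the location under the cursor.
; A cursor target task supplies the location, draws a debug sphere there and turns the avatar to face it through CombatInterface.
; It plays the cast montage and spawns the projectile when the montage's gameplay event arrives.
; The ability ends shortly after spawning, or when the montage completes, blends out, is interrupted or is cancelled.
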(event Ability|EventActivateAbility
  (bind _gameplayabilitytargetdatahandle (|CursorTargetProxy)
    (:then
      (|PlayMontageandWaitProxy "None" "/Game/Assets/Characters/Aura/Animations/Abilities/AM_Cast_FireBolt.AM_Cast_FireBolt" 1.0 "None" false 1.0 0.0 false
        (:then
          (Ability|Tasks|WaitGameplayEvent "(TagName=\"Event.Montage.FireBolt\")" 0
            (:EventReceived
              (Class|AuraProjectileSpell|SpawnProjectile (Variables|Default|GetProjectileTargetLocation))
              (Utilities|FlowControl|Delay 0.6))))
        (:OnCompleted
          _)
        (:OnBlendOut
          _)
        (:OnInterrupted
          _)
        (:OnCancelled
          _))
      (Ability|EndAbility))
    (:OnCursorTarget
      (bind _output_get (Variables|Default|SetProjectileTargetLocation (.Location (Collision|BreakHitResult (Ability|TargetData|GetHitResultfromTargetData _gameplayabilitytargetdatahandle)))))
      (Rendering|Debug|DrawDebugSphere _output_get 8.0 12 "(R=1.000000,G=0.000000,B=0.037457,A=1.000000)" 2.0 1.0)
      (bind _ascombat_interface (Utilities|Casting|CastToCombatInterface (Ability|GetAvatarActorfromActorInfo)))
      (Class|CombatInterface|SetFacingTarget _ascombat_interface (Variables|Default|GetProjectileTargetLocation)))))

(event Ability|EventOnEndAbility
  (params (bWasCancelled :type Boolean)))