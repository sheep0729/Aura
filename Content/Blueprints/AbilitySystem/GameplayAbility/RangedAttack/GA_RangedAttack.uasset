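; GA_RangedAttack is a gameplay ability that makes the avatar fire a projectile at its current combat target.
; It turns the avatar toward the target and plays a random tagged montage from its CombatInterface.
; A gameplay event matching the montage's tag triggers SpawnProjectile with the montage's socket tag and the target's location.
; The ability ends when the montage completes, is interrupted or cancelled, or when no valid target exists.
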(event Ability|EventActivateAbility
  (bind _output_get (Variables|Default|SetAvatar%20Actor (Ability|GetAvatarActorfromActorInfo)))
  (bind _returnvalue (Class|EnemyInterface|GetCombatTarget(Message) _output_get))
  (bind _output_get_2 (Variables|Default|SetCombat%20Target _returnvalue))
  (Utilities|IsValid _output_get_2
    (:Is%20Valid
      (Class|CombatInterface|SetFacingTarget(Message) (Variables|Default|GetAvatar%20Actor) (Transformation|GetActorLocation _output_get_2))
      (bind _ascombat_interface (Utilities|Casting|CastToCombatInterface (Variables|Default|GetAvatar%20Actor)))
      (bind _outmontages (Class|CombatInterface|GetMontages _ascombat_interface))
      (bind _output_get_3 (Variables|Default|SetSelected%20Tagged%20Montage (.OutItem (Utilities|Array|Random _outmontages))))
      (|PlayMontageandWaitProxy "None" (.Montage (Utilities|Struct|BreakTaggedMontage _output_get_3)) 1.0 "None" false 1.0 0.0 true
        (:then
          (Ability|Tasks|WaitGameplayEvent (.MontageTag (Utilities|Struct|BreakTaggedMontage (Variables|Default|GetSelected%20Tagged%20Montage))) 0
            (:EventReceived
              (Class|AuraProjectileSpell|SpawnProjectile (Transformation|GetActorLocation (Variables|Default|GetCombat%20Target)) (.SocketTag (Utilities|Struct|BreakTaggedMontage (Variables|Default|GetSelected%20Tagged%20Montage)))))))
        (:OnCompleted
          (Ability|EndAbility :!label _label) ; 不连接 Blend Out 就一定要选上 Allow Interrupt After Blend Out ，否则会导致技能无法结束
        )
        (:OnInterrupted
          (goto _label))
        (:OnCancelled
          (goto _label))))
    (:Is%20Not%20Valid
      (Ability|EndAbility))))