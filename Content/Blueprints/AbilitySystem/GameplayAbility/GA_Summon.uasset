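; Gameplay ability that lets a shaman avatar summon minions around itself during a summon montage.
; On the montage's attack event tag, it shows ground Niagara effects at shuffled spawn locations, then after a short delay spawns a random minion class at each, facing away from the summoner.
; Each minion gets a default controller and updates the avatar's minion count on spawn and destruction.
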(event Custom|OnDestroyed_Event
  (params (DestroyedActor :type Actor%20Object%20Reference))
  (Class|CombatInterface|IncrementMinionCount(Message) (Ability|GetAvatarActorfromActorInfo) -1))

(event Ability|EventActivateAbility
  (bind _returnvalue (Ability|GetAvatarActorfromActorInfo))
  (Variables|Default|SetSpawnLocationIndex 0)
  (bind _returnvalue_2 (Class|GASummon|GetSpawnLocations))
  (bind _output_get (Variables|Default|SetSpawnLocations _returnvalue_2))
  (Utilities|Array|Shuffle _output_get)
  (|PlayMontageandWaitProxy "None" "/Game/Assets/Enemies/Shaman/Animations/AM_Shaman_Summon.AM_Shaman_Summon" 1.0 "None" false 1.0 0.0 true
    (:then
      (Ability|Tasks|WaitGameplayEvent "(TagName=\"Montage.Attack.1\")" 0
        (:EventReceived
          (for _array_element (Variables|Default|GetSpawnLocations)
            (Niagara|SpawnSystematLocation "/Game/Assets/Effects/Combat/NS_GroundSummon.NS_GroundSummon" _array_element))
          (Utilities|FlowControl|Delay 1.0)
          (for _array_element_2 (Variables|Default|GetSpawnLocations)
            (bind _aspawn (Utilities|Casting|CastToPawn _returnvalue))
            (bind _returnvalue_3 (Game|SpawnActorfromClass (Class|GASummon|GetRandomMinionClass) (Math|Transform|MakeTransform (+ _array_element_2 "0.000000,0.000000,70.000000") (Math|Rotator|FindLookatRotation (Transformation|GetActorLocation _returnvalue) (+ _array_element_2 "0.000000,0.000000,70.000000")) "1.000000,1.000000,1.000000") "AdjustIfPossibleButAlwaysSpawn" "MultiplyWithRoot" 0 _aspawn))
            (Game|AssignOnDestroyed _returnvalue_3 (delegate Custom|OnDestroyed_Event))
            (Pawn|SpawnDefaultController _returnvalue_3)
            (Class|CombatInterface|IncrementMinionCount(Message) (Ability|GetAvatarActorfromActorInfo) 1))
          (Ability|EndAbility))))))