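; Gameplay Ability for melee attacks: faces the avatar toward its combat target and plays a random tagged montage from its CombatInterface.
; The montage's gameplay event supplies target data; non-friendly actors take damage and a blood cue.
; Any hit fires an impact cue with the montage's sound and ends the ability, leaving the montage playing.
; The ability also ends without a valid target or montage, or when the montage finishes or is interrupted.
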(event Ability|EventActivateAbility
  (bind _output_get (Variables|Default|SetAvatar%20Actor (Ability|GetAvatarActorfromActorInfo)))
  (if (Ability|HasAuthority _output_get)
    (Development|PrintText "Running [GA_MeleeAttack] on [Server]")
    (else
      (Development|PrintText "Running [GA_MeleeAttack] on [Client]")))
  (bind _returnvalue (Class|EnemyInterface|GetCombatTarget(Message) (Variables|Default|GetAvatar%20Actor)))
  (Utilities|IsValid _returnvalue
    (:Is%20Valid
      (bind _ascombat_interface (Utilities|Casting|CastToCombatInterface (Variables|Default|GetAvatar%20Actor))
        (:then
          (bind _output_get_2 (Variables|Default|SetCombat%20Interface _ascombat_interface))
          (Class|CombatInterface|SetFacingTarget _output_get_2 (Transformation|GetActorLocation _returnvalue))
          (bind _outmontages (Class|CombatInterface|GetMontages (Variables|Default|GetCombat%20Interface)))
          (bind _output_get_3 (Variables|Default|SetMontages _outmontages))
          (Variables|Default|SetSelectedTaggedMontage (.OutItem (Utilities|Array|Random _output_get_3)))
          (if (Utilities|Array|IsNotEmpty (Variables|Default|GetMontages))
            (Variables|Default|SetSelected%20Montage%20Tag (.MontageTag (Utilities|Struct|BreakTaggedMontage (Variables|Default|GetSelectedTaggedMontage))))
            (Variables|Default|SetSelected%20Socket%20Tag (.SocketTag (Utilities|Struct|BreakTaggedMontage (Variables|Default|GetSelectedTaggedMontage))))
            (Variables|Default|SetImpact%20Sound (.ImpactSound (Utilities|Struct|BreakTaggedMontage (Variables|Default|GetSelectedTaggedMontage))))
            (|PlayMontageandWaitProxy "None" (.Montage (Utilities|Struct|BreakTaggedMontage (Variables|Default|GetSelectedTaggedMontage))) 1.0 "None" false 1.0 0.0 false
              (:then
                (bind _payload (Ability|Tasks|WaitGameplayEvent (Variables|Default|GetSelected%20Montage%20Tag) 0)
                  (:EventReceived
                    (for _array_element (Ability|TargetData|GetAllActorsfromTargetData (Utilities|Struct|BreakGameplayEventData _payload))
                      (if (Class|AuraAbilitySystemLibrary|IsNotFriends _array_element (Ability|GetAvatarActorfromActorInfo))
                        (bind _output_get_4 (Variables|Default|SetTargetActor _array_element))
                        (Class|DamageGameplayAbility|CauseDamage _output_get_4)
                        (GameplayCue|ExecuteGameplayCueOnActor(Burst) (Variables|Default|GetTargetActor) "(TagName=\"GameplayCue.BloodEffect\")" (Ability|GameplayCue|MakeGameplayCueParameters :Location (Transformation|GetActorLocation (Variables|Default|GetTargetActor))))))
                    (if (Utilities|Array|IsNotEmpty (Ability|TargetData|GetAllActorsfromTargetData (Utilities|Struct|BreakGameplayEventData _payload)))
                      (Class|GameplayAbility|ExecuteGameplayCuewithParams "(TagName=\"GameplayCue.MeleeImpact\")" (Ability|GameplayCue|MakeGameplayCueParameters :Location (Class|AbilitySystemBlueprintLibrary|GetTargetDataEndPoint (Utilities|Struct|BreakGameplayEventData _payload)) :SourceObject (Variables|Default|GetImpact%20Sound)))
                      (Ability|EndAbility)))))
              (:OnCompleted
                (Ability|EndAbility :!label _label))
              (:OnBlendOut
                (goto _label))
              (:OnInterrupted
                (goto _label))
              (:OnCancelled
                (goto _label)))
            (else
              (Ability|EndAbility))))
        (:CastFailed
          (Ability|EndAbility :!label _label_2))))
    (:Is%20Not%20Valid
      (goto _label_2))))

(event Ability|EventOnEndAbility
  (params (bWasCancelled :type Boolean)))