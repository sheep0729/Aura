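; AN_MontageEvent is an anim notify that sends a gameplay event with its EventTag to the owning AuraCharacterBase, signalling the ability system from an animation.
; For Warriors with authority, it finds live players within a small sphere at the SocketTag combat socket, excluding the owner, and attaches them as target data.
; That path also draws a debug sphere at the attack origin.
; All other cases send the tag without target data.
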(fn ReceivedNotify
  (params (MeshComp :type Skeletal%20Mesh%20Component%20Object%20Reference) (Animation :type Anim%20Sequence%20Base%20Object%20Reference) (EventReference :type Anim%20Notify%20Event%20Reference%20Structure%20%28by%20ref%29))
  (bind _asaura_character_base (Utilities|Casting|CastToAuraCharacterBase (Components|GetOwner MeshComp)))
  (bind _output_get (LocalVariables|SetOwner%20Character _asaura_character_base))
  (if (and (Utilities|Enum|Equal(Enum) (Variables|/Script/Aura.AuraCharacterBase|GetCharacterClass _output_get) "Warrior") (Ability|HasAuthority (LocalVariables|GetOwner%20Character)))
    (bind _returnvalue (Class|CombatInterface|GetCombatSocketLocation(Message) (LocalVariables|GetOwner%20Character) (Variables|Default|GetSocketTag)))
    (bind _output_get_2 (LocalVariables|SetAttack%20Origin _returnvalue))
    (Rendering|Debug|DrawDebugSphere _output_get_2 45.0 12 "(R=1.000000,G=1.000000,B=1.000000,A=1.000000)" 1.0 1.0)
    (bind _outoverlappingactors (Class|AuraAbilitySystemLibrary|GetLivePlayerWithinRadius (LocalVariables|GetOwner%20Character) (Utilities|Array|MakeArray (LocalVariables|GetOwner%20Character)) 45.0 (LocalVariables|GetAttack%20Origin)))
    (Ability|SendGameplayEventtoActor (LocalVariables|GetOwner%20Character) (Variables|Default|GetEventTag) (Utilities|Struct|MakeGameplayEventData (Ability|TargetData|AbilityTargetDatafromActorArray _outoverlappingactors)))
    (return true)
    (else
      (Ability|SendGameplayEventtoActor (LocalVariables|GetOwner%20Character) (Variables|Default|GetEventTag))
      (return true))))