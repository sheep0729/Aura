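; BP_FlamePillar is a flame pillar actor whose fire light flickers continuously.
; On BeginPlay it starts a timeline that scales the FireLight intensity from a base value along a flame intensity track.
; Each time the timeline finishes, it sets a new time and restarts, with a random float fed into the timeline to vary the flicker.
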(event Custom|Start%20TimeLine
  (bind _flame_intensity (Timeline|Flame%20Intensity%20Timeline Play)
    (:Update
      (Rendering|Components|Light|SetIntensity (Variables|Default|GetFireLight) (* (+ _flame_intensity 0.0) (Variables|Default|GetBase%20Flame%20Intensity))))
    (:Finished
      (CallFunction|SetNewTime)
      (CallFunction|StartTimeLine))))

(event Custom|Set%20New%20Time
  (bind _flame_intensity (Timeline|Flame%20Intensity%20Timeline SetNewTime)
    (:Update
      (Rendering|Components|Light|SetIntensity (Variables|Default|GetFireLight) (* (+ _flame_intensity 0.0) (Variables|Default|GetBase%20Flame%20Intensity))))
    (:Finished
      (CallFunction|SetNewTime)
      (CallFunction|StartTimeLine))))

(event EventBeginPlay
  (CallFunction|StartTimeLine))

(fn ConstructionScript)