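; BP_FadeActor is an actor whose mesh fades out and back in by animating a "Fade" material parameter.
; Construction caches original materials and builds dynamic instances from FadeMaterialInstances, which BeginPlay applies at full Fade.
; FadeOut plays a timeline and Fadein reverses it, driving the parameter and switching a custom collision channel between Block and Ignore at a threshold.
; ResetMaterials can restore the originals but is not called here.
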(event EventBeginPlay
  (CallFunction|SetMaterialstoDynamicInstances)
  (for _array_element (Variables|Default|GetDynamic%20Material%20Instances)
    (Rendering|Material|SetScalarParameterValue _array_element "Fade" 1.0 :!class /Script/Engine.MaterialInstanceDynamic)))

(event Collision|EventActorBeginOverlap
  (params (OtherActor :type Actor%20Object%20Reference)))

(event EventTick
  (params (DeltaSeconds :type Float%20%28single-precision%29)))

(event EventFadeOut
  (bind _mesh (Variables|Default|GetMesh))
  (bind _fade (Timeline|Fade%20Timeline Play)
    (:Update
      (for _array_element (Variables|Default|GetDynamic%20Material%20Instances)
        (Rendering|Material|SetScalarParameterValue _array_element "Fade" _fade :!class /Script/Engine.MaterialInstanceDynamic)
        (if (>= _fade 0.8)
          (Collision|SetCollisionResponsetoChannel _mesh "ECC_GameTraceChannel3" "ECR_Block")
          (else
            (Collision|SetCollisionResponsetoChannel _mesh "ECC_GameTraceChannel3" "ECR_Ignore")))))))

(event EventFadein
  (bind _mesh (Variables|Default|GetMesh))
  (bind _fade (Timeline|Fade%20Timeline Reverse)
    (:Update
      (for _array_element (Variables|Default|GetDynamic%20Material%20Instances)
        (Rendering|Material|SetScalarParameterValue _array_element "Fade" _fade :!class /Script/Engine.MaterialInstanceDynamic)
        (if (>= _fade 0.8)
          (Collision|SetCollisionResponsetoChannel _mesh "ECC_GameTraceChannel3" "ECR_Block")
          (else
            (Collision|SetCollisionResponsetoChannel _mesh "ECC_GameTraceChannel3" "ECR_Ignore")))))))

(fn ConstructionScript
  (Utilities|Array|Clear (Variables|Default|GetDynamic%20Material%20Instances))
  (Variables|Default|SetOriginal%20Materials (Rendering|Material|GetMaterials (Variables|Default|GetMesh)))
  (for _array_element (Variables|Default|GetFade%20Material%20Instances)
    (bind _returnvalue (Rendering|Material|CreateDynamicMaterialInstance _array_element "None" "None" :!class /Script/Engine.KismetMaterialLibrary))
    (Utilities|Array|AddUnique (Variables|Default|GetDynamic%20Material%20Instances) _returnvalue)))

(fn SetMaterialstoDynamicInstances
  (for (_array_element _array_index) (Variables|Default|GetDynamic%20Material%20Instances)
    (Rendering|Material|SetMaterial (Variables|Default|GetMesh) _array_index _array_element)))

(fn ResetMaterials
  (for (_array_element _array_index) (Variables|Default|GetOriginal%20Materials)
    (Rendering|Material|SetMaterial (Variables|Default|GetMesh) _array_index _array_element)))